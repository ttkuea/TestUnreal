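; YBar is an actor that slides back and forth along a referenced spline while the Motor's I or K key is held.
; On BeginPlay it snaps to the spline start and plays a timeline that serves as its update loop.
; Each update steps it by a fixed, frame-based amount along the first point's direction, treating the path as straight.
; Travel limits compare only world X against spline points 2 and -1.
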(event `self.ReceiveBeginPlay`
  (bind _returnvalue (`SplineComponent.GetLocationAtDistanceAlongSpline` (`/Game/Blueprints/XGantry.CoreSpline` (`self.SplineRef`)) 0.0 "World"))
  (bind _returnvalue_2 (`SplineComponent.GetLocationAtSplinePoint` (`/Game/Blueprints/XGantry.CoreSpline` (`self.SplineRef`)) -1 "World"))
  (bind _returnvalue_3 (`SplineComponent.GetLocationAtSplinePoint` (`/Game/Blueprints/XGantry.CoreSpline` (`self.SplineRef`)) 2 "World"))
  (bind _returnvalue_4 (+ (`SceneComponent.K2_GetComponentLocation` (`self.DefaultSceneRoot`)) (* (`SplineComponent.GetDirectionAtSplinePoint` (`/Game/Blueprints/XGantry.CoreSpline` (`self.SplineRef`)) 0 "World") -2)))
  (bind _returnvalue_5 (+ (`SceneComponent.K2_GetComponentLocation` (`self.DefaultSceneRoot`)) (* (`SplineComponent.GetDirectionAtSplinePoint` (`/Game/Blueprints/XGantry.CoreSpline` (`self.SplineRef`)) 0 "World") 2)))
  (`self.K2_SetActorLocation` _returnvalue false true)
  (set `self.CurVec` _returnvalue)
  (`Timeline|Update Timeline`
    (:`Update`
      (if (`/Game/Blueprints/MotorCylinder.isIHeld` (`self.Motor`))
        (if (> (.x _returnvalue_5) (.x _returnvalue_3))
          (set `self.CurVec` _returnvalue_3)
          (else
            (set `self.CurVec` _returnvalue_5)))
        (`self.K2_SetActorLocation` (`self.CurVec`))
        (elif (`/Game/Blueprints/MotorCylinder.isKHeld` (`self.Motor`))
          (if (< (.x _returnvalue_4) (.x _returnvalue_2))
            (set `self.CurVec` _returnvalue_2)
            (else
              (set `self.CurVec` _returnvalue_4)))
          (`self.K2_SetActorLocation` (`self.CurVec`)))))))

(fn `UserConstructionScript`)