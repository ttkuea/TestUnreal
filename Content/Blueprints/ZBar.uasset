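; ZBar is the vertical bar of a gantry claw, moved horizontally by player input and lowered on command.
; On BeginPlay it snaps to the spline start, then a timeline steps it along two spline directions from Motor's I/J/K/L held flags, clamping at spline end points.
; O, gated by IsRetracted, runs timelines that lower the Cylinder and, after a delay, raise it.
; The U "Claw Up" handler has no effect.
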(event `Key|U`
  (params (Key :type "Key Structure"))
  ;[1 1 1] Claw Up
  (:`Pressed`
    (if (`self.isRetracted`)
      _)))

(event `Key|O`
  (params (Key :type "Key Structure"))
  ;[1 1 1] Claw Down
  (:`Pressed`
    (if (`self.isRetracted`)
      (`Timeline|Gantry Up` :!via `PlayFromStart`
        (:`Update`
          (`SceneComponent.K2_AddLocalOffset` (`self.Cylinder`) (0.0 0.0 -1.0) false false)
          (set `self.isRetracted` false)
          (`KismetSystemLibrary.Delay` 2.5)
          ;[1 1 1] Claw Up
          (`Timeline|Timeline_1` :!via `PlayFromStart`
            (:`Update`
              (`SceneComponent.K2_AddLocalOffset` (`self.Cylinder`) (0.0 0.0 1.0) false false)
              (set `self.isRetracted` true))))))))

(event `self.ReceiveBeginPlay`
  (bind _returnvalue (`SplineComponent.GetLocationAtDistanceAlongSpline` (`/Game/Blueprints/XGantry.CoreSpline` (`self.SplineRef`)) 0.0 "World"))
  (bind _returnvalue_2 (`SplineComponent.GetLocationAtSplinePoint` (`/Game/Blueprints/XGantry.CoreSpline` (`self.SplineRef`)) 2 "World"))
  (bind _returnvalue_3 (`SplineComponent.GetLocationAtSplinePoint` (`/Game/Blueprints/XGantry.CoreSpline` (`self.SplineRef`)) 0 "World"))
  (bind _x (.x (`SplineComponent.GetLocationAtSplinePoint` (`/Game/Blueprints/XGantry.CoreSpline` (`self.XSplineRef`)) 0 "World")))
  (bind _x_2 (.x (`SplineComponent.GetLocationAtSplinePoint` (`/Game/Blueprints/XGantry.CoreSpline` (`self.XSplineRef`)) 2 "World")))
  (bind _returnvalue_4 (+ (`SceneComponent.K2_GetComponentLocation` (`self.DefaultSceneRoot`)) (* (`SplineComponent.GetDirectionAtSplinePoint` (`/Game/Blueprints/XGantry.CoreSpline` (`self.SplineRef`)) 0 "World") -2)))
  (bind _returnvalue_5 (+ (`SceneComponent.K2_GetComponentLocation` (`self.DefaultSceneRoot`)) (* (`SplineComponent.GetDirectionAtSplinePoint` (`/Game/Blueprints/XGantry.CoreSpline` (`self.SplineRef`)) 0 "World") 2)))
  (bind _returnvalue_6 (+ (`SceneComponent.K2_GetComponentLocation` (`self.DefaultSceneRoot`)) (* (`SplineComponent.GetDirectionAtSplinePoint` (`/Game/Blueprints/XGantry.CoreSpline` (`self.XSplineRef`)) 0 "World") -2)))
  (bind _returnvalue_7 (+ (`SceneComponent.K2_GetComponentLocation` (`self.DefaultSceneRoot`)) (* (`SplineComponent.GetDirectionAtSplinePoint` (`/Game/Blueprints/XGantry.CoreSpline` (`self.XSplineRef`)) 0 "World") 2)))
  ;[1 1 1] Main
  (`self.EnableInput` (`GameplayStatics.GetPlayerController` 0))
  (set `self.isRetracted` true)
  (`self.K2_SetActorLocation` _returnvalue false true)
  (set `self.CurVecs` _returnvalue)
  (`Timeline|Timeline_0`
    (:`Update`
      (`|ExecutionSequence`
        (:`then_0`
          (if (`/Game/Blueprints/MotorCylinder.isIHeld` (`self.Motor`))
            ;[1 1 1] I
            (if (> (.x _returnvalue_7) _x_2)
              (set `self.CurVecs` (`KismetMathLibrary.MakeVector` _x_2 (.y _returnvalue_7) (.z (`SplineComponent.GetLocationAtSplinePoint` (`/Game/Blueprints/XGantry.CoreSpline` (`self.XSplineRef`)) 2 "World"))))
              (else
                (set `self.CurVecs` _returnvalue_7)))
            (`self.K2_SetActorLocation` (`self.CurVecs`))
            (elif (`/Game/Blueprints/MotorCylinder.isKHeld` (`self.Motor`))
              ;[1 1 1] K
              (if (< (.x _returnvalue_6) _x)
                (set `self.CurVecs` (`KismetMathLibrary.MakeVector` _x (.y _returnvalue_6) (.z _returnvalue_6)))
                (else
                  (set `self.CurVecs` _returnvalue_6)))
              (`self.K2_SetActorLocation` (`self.CurVecs`)))))
        (:`then_1`
          (if (`/Game/Blueprints/MotorCylinder.isJHeld` (`self.Motor`))
            ;[1 1 1] J
            (if (< (.y _returnvalue_4) (.y _returnvalue_3))
              (set `self.CurVecs` _returnvalue_3)
              (else
                (set `self.CurVecs` _returnvalue_4)))
            (`self.K2_SetActorLocation` (`self.CurVecs`))
            (elif (`/Game/Blueprints/MotorCylinder.isLHeld` (`self.Motor`))
              ;[1 1 1] L
              (if (> (.y _returnvalue_5) (.y _returnvalue_2))
                (set `self.CurVecs` _returnvalue_2)
                (else
                  (set `self.CurVecs` _returnvalue_5)))
              (`self.K2_SetActorLocation` (`self.CurVecs`)))))))))

(fn `UserConstructionScript`)