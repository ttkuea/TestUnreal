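; MotorCylinder is an actor that rotates about one local axis under keyboard control.
; It enables input from the first player controller and tracks held flags for the I, K, J and L keys.
; A timeline started at BeginPlay applies a fixed rotation step per update, forward for I and backward for K, with I taking priority and no delta-time scaling.
; The J and L flags are set but never read.
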(event `Key|L`
  (params (Key :type "Key Structure"))
  (:`Pressed`
    (set `self.isLHeld` true))
  (:`Released`
    (set `self.isLHeld` false)))

(event `Key|I`
  (params (Key :type "Key Structure"))
  (:`Pressed`
    (set `self.isIHeld` true))
  (:`Released`
    (set `self.isIHeld` false)))

(event `Key|K`
  (params (Key :type "Key Structure"))
  (:`Pressed`
    (set `self.isKHeld` true))
  (:`Released`
    (set `self.isKHeld` false)))

(event `Key|J`
  (params (Key :type "Key Structure"))
  (:`Pressed`
    (set `self.isJHeld` true))
  (:`Released`
    (set `self.isJHeld` false)))

(event `self.ReceiveBeginPlay`
  (`self.EnableInput` (`GameplayStatics.GetPlayerController` 0))
  (`Timeline|Update Timeline`
    (:`Update`
      (if (`self.isIHeld`)
        (`self.K2_AddActorLocalRotation` (struct :`Yaw` 10.0))
        (elif (`self.isKHeld`)
          (`self.K2_AddActorLocalRotation` (struct :`Yaw` -10.0)))))))

(fn `UserConstructionScript`)